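; BP_GameModePacman is the game mode for a Pac-Man game, handling the win and lose conditions.
; Every Tick it switches on Lives: zero plays the death sound, pauses the game and shows DeadUI.
; Otherwise, a truncated TotalScore of exactly 2550 shows WinUI and sets paused to false, so the game keeps running.
; The win branch has no one-shot guard, so it creates another widget each tick the score matches.
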(event EventBeginPlay)

(event EventTick
  (params (DeltaSeconds :type Float%20%28single-precision%29))
  (switch int (Variables|Default|GetLives)
    (:Default
      (switch int (Math|Float|Truncate (Variables|Default|GetTotalScore))
        (:2550
          (Game|SetGamePaused false)
          (bind _returnvalue (UserInterface|CreateWidget "/Game/UI/WinUI.WinUI_C"))
          (UserInterface|Viewport|AddtoViewport _returnvalue 0))))
    (:0
      (Audio|PlaySound2D "/Game/Sounds/pacman_death.pacman_death" 1.0 1.0 0.0 0 0)
      (Game|SetGamePaused true)
      (bind _returnvalue_2 (UserInterface|CreateWidget "/Game/UI/DeadUI.DeadUI_C"))
      (UserInterface|Viewport|AddtoViewport _returnvalue_2 0))))

(fn ConstructionScript)